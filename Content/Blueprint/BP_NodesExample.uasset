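; Example actor demonstrating custom Blueprint nodes for array sorting, timers, coroutines, config values and view focusing.
; Number keys sort random student structs by comparator function or property name, and write or read config variables.
; Other keys spawn 500 cubes, rotate them with pausable per-object timers and offset them via coroutines as a Tick alternative.
; BeginPlay binds StaticMeshActor clicks to move the pawn to frame the actor; unwired nodes form a reference palette.
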(event Custom|OnClickActor
  (params (TouchedActor :type Actor%20Object%20Reference) (ButtonPressed :type Key%20Structure :default "None"))
  ;[0.9062 0.1647 1] Focus node examples
  ;;[1 1 1] Focus Actor
  (bind _returnvalue (Class|BlueprintProLibrary|GetViewportTransformfromActors (Utilities|Array|MakeArray TouchedActor) 1.0)) ; If you add several  actors, it'll focus on all actors.
  (Transformation|SetActorTransform (Game|Player|GetPlayerPawn 0) _returnvalue false true)
  (Pawn|SetControlRotation (Game|GetPlayerController 0) (.Rotation (Math|Transform|BreakTransform _returnvalue))))

(event Custom|OnClickComponent
  (params (TouchedComponent :type Primitive%20Component%20Object%20Reference) (ButtonPressed :type Key%20Structure :default "None"))
  ;[0.9062 0.1647 1] Focus node examples
  ;;[1 1 1] Focus Component
  (bind _returnvalue (Class|BlueprintProLibrary|GetViewportTransformfromActorsandComponents (Utilities|Array|MakeArray 0) (Utilities|Array|MakeArray TouchedComponent) 1.0)) ; Can focus on both Actors and Components simultaneously
  (Transformation|SetActorTransform (Game|Player|GetPlayerPawn 0) _returnvalue false true)
  (Pawn|SetControlRotation (Game|GetPlayerController 0) (.Rotation (Math|Transform|BreakTransform _returnvalue))))

(event EventBeginPlay
  (bind _returnvalue (Game|GetPlayerController 0))
  ;[0.9062 0.1647 1] Focus node examples
  (Input|EnableInput _returnvalue)
  (Variables|/Script/Engine.PlayerController|SetbShowMouseCursor _returnvalue true)
  (Variables|/Script/Engine.PlayerController|SetbEnableClickEvents _returnvalue true) ; Warning：Enable Click events
  (Collision|SetActorEnableCollision (Game|Player|GetPlayerPawn 0) false) ; Optional
  ;;[1 1 1] Focus Actor
  (bind _outactors (Actor|GetAllActorsOfClass "/Script/Engine.StaticMeshActor"))
  (bind _output_get (Variables|Default|SetStaticMeshActors _outactors))
  (for _array_element _output_get
    (EventDispatchers|BindEventtoOnClicked _array_element (delegate Custom|OnClickActor))))

(event Input|KeyboardEvents|6
  (params (Key :type Key%20Structure :default "None"))
  ;[0.0469 0.7135 1] Async node_Simple Coroutine,  alternative to the Tick Event
  (:Pressed
    (for _array_element (Variables|SETTIMER|GetMovableActors)
      (bind (_referenceobject _progress) (|Coroutine _array_element (Math|Random|RandomFloatinRange 0.0 2.0) (Math|Random|RandomFloatinRange 2.0 1e+01))
        (:Update
          (bind _asactor (Utilities|Casting|CastToActor _referenceobject))
          (Transformation|AddLocalOffset (Variables|/Script/Engine.Actor|GetRootComponent _asactor) (Math|Vector|MakeVector 0.0 (Math|Float|Lerp -5e+01 5e+01 _progress) 0.0) false false))))))

(event Input|KeyboardEvents|3
  (params (Key :type Key%20Structure :default "None"))
  ;[0.0469 0.7135 1] SetTimer Node example: simultaneously controlling the rotation of N actors
  ;;[1 1 1] Spawn Actor for some tests
  (:Pressed
    (for _index (range 0 500)
      (bind _returnvalue (Game|SpawnActorfromClass "/Script/Engine.StaticMeshActor" (Math|Transform|MakeTransform (* (Math|Random|RandomUnitVector) (Math|Float|MakeLiteralFloat 3e+03))) "AlwaysSpawn" 0 0))
      (Transformation|SetMobility _returnvalue "Movable")
      (Components|StaticMesh|SetStaticMesh (Variables|/Script/Engine.StaticMeshActor|GetStaticMeshComponent _returnvalue) "/Engine/BasicShapes/Cube.Cube")
      (Utilities|Array|Add (Variables|SETTIMER|GetMovableActors) _returnvalue))))

(event Input|KeyboardEvents|7
  (params (Key :type Key%20Structure :default "None"))
  (bind _returnvalue (Class|ConfigFunctionLibrary|GetDefaultSectionName))
  (bind _myfloatvariable (Variables|BP_CONFIG|GetMyFloatVariable))
  (bind _mystringvariable (Variables|BP_CONFIG|GetMyStringVariable))
  (bind _myintvariable (Variables|BP_CONFIG|GetMyIntVariable))
  ;[0.5533 1 0.3332] Set config value
  (:Pressed
    (Class|ConfigFunctionLibrary|SetConfigPorpertybyName _returnvalue (Class|ConfigFunctionLibrary|GetPropertyName _myintvariable) false "DefaultProject.ini" _myintvariable)
    (Class|ConfigFunctionLibrary|SetConfigPorpertybyName _returnvalue (Class|ConfigFunctionLibrary|GetPropertyName _myfloatvariable) false "DefaultProject.ini" _myfloatvariable)
    (Class|ConfigFunctionLibrary|SetConfigPorpertybyName _returnvalue (Class|ConfigFunctionLibrary|GetPropertyName _mystringvariable) false "DefaultProject.ini" _mystringvariable)))

(event Input|KeyboardEvents|8
  (params (Key :type Key%20Structure :default "None"))
  (bind _returnvalue (Class|ConfigFunctionLibrary|GetDefaultSectionName))
  (bind _myintvariable (Variables|BP_CONFIG|GetMyIntVariable))
  (bind _myfloatvariable (Variables|BP_CONFIG|GetMyFloatVariable))
  (bind _mystringvariable (Variables|BP_CONFIG|GetMyStringVariable))
  (bind _returnvalue_2 (Class|ConfigFunctionLibrary|GetPropertyName _myintvariable))
  (bind _returnvalue_3 (Class|ConfigFunctionLibrary|GetPropertyName _mystringvariable))
  (bind _returnvalue_4 (Class|ConfigFunctionLibrary|GetPropertyName _myfloatvariable))
  ;[0.5533 1 0.3332] Get config value
  (:Pressed
    (Utilities|FlowControl|Sequence
      (:then_0
        (bind (_bsuccessful _value) (Class|ConfigFunctionLibrary|GetConfigPorpertybyName _returnvalue _returnvalue_4))
        (Development|PrintString (Utilities|String|Append "Get  config value： " _returnvalue_4 ",  " (Utilities|String|ToString(Float) _value) "， " (Utilities|String|ToString(Boolean) _bsuccessful)) true true "(R=0.226079,G=1.000000,B=0.000000,A=1.000000)" 1e+01))
      (:then_1
        (bind (_bsuccessful_2 _value_2) (Class|ConfigFunctionLibrary|GetConfigPorpertybyName _returnvalue _returnvalue_2))
        (Development|PrintString (Utilities|String|Append "Get  config value： " _returnvalue_2 ",  " (Utilities|String|ToString(Integer) _value_2) "， " (Utilities|String|ToString(Boolean) _bsuccessful_2)) true true "(R=0.182687,G=0.014812,B=1.000000,A=1.000000)" 1e+01))
      (:then_2
        (bind (_bsuccessful_3 _value_3) (Class|ConfigFunctionLibrary|GetConfigPorpertybyName _returnvalue _returnvalue_3))
        (Development|PrintString (Utilities|String|Append "Get  config value： " _returnvalue_3 ",  " _value_3 "， " (Utilities|String|ToString(Boolean) _bsuccessful_3)) true true "(R=0.000000,G=0.660000,B=1.000000,A=1.000000)" 1e+01)))))

(event Input|KeyboardEvents|5
  (params (Key :type Key%20Structure :default "None"))
  ;[0.0469 0.7135 1] SetTimer Node example: simultaneously controlling the rotation of N actors
  ;;[1 1 1] Pause/Unpause Timer
  (:Pressed
    (bind _isa (Utilities|FlowControl|FlipFlop)
      (:A
        _)
      (:B
        _))
    (Development|PrintString (Utilities|String|SelectString "Pause Timer" "Unpause Timer" _isa))
    (bind _keys (Utilities|Map|Keys (Variables|SET_TIMER|GetActorsTimerHandle)))
    (for _array_element _keys
      (if _isa
        (Utilities|Time|PauseTimerbyHandle _array_element)
        (else
          (Utilities|Time|UnpauseTimerbyHandle _array_element))))))

(event Input|KeyboardEvents|2
  (params (Key :type Key%20Structure :default "None"))
  (bind _mystructarray (Variables|ARRAY|GetMyStructArray))
  ;[0.1393 1 0.9303] example: Array Sort by Property Name
  (:Pressed
    (Utilities|Array|Clear _mystructarray)
    (for _index (range 0 100)
      (Utilities|Array|Add _mystructarray (Utilities|Struct|MakeFStudent "None" _index (Math|Random|RandomFloatinRange 1.5e+02 2e+02) (Math|Random|RandomFloatinRange 1.5e+02 2e+02) (Math|Random|RandomFloatinRange 0.0 1e+02))))
    (|ArraySort _mystructarray "Height" true) ; Array Sort By Property
    (for (_array_element _array_index) _mystructarray
      (Development|PrintString (Utilities|String|Append (Utilities|String|ToString(Integer) _array_index) ": " (Utilities|String|ToString(Float) (.height _array_element)) ", " (Utilities|String|ToString(Float) (.bodyweight _array_element)) ", " (Utilities|String|ToString(Float) (.score _array_element)))))))

(event Input|KeyboardEvents|1
  (params (Key :type Key%20Structure :default "None"))
  (bind _mystructarray (Variables|ARRAY|GetMyStructArray))
  ;[0.1393 1 0.9303] example: Array Sort By  Blueprint function
  (:Pressed
    (Utilities|Array|Clear _mystructarray)
    (for _index (range 0 100)
      (Utilities|Array|Add _mystructarray (Utilities|Struct|MakeFStudent "None" _index (Math|Random|RandomFloatinRange 1.5e+02 2e+02) (Math|Random|RandomFloatinRange 1.5e+02 2e+02) (Math|Random|RandomFloatinRange 0.0 1e+02))))
    (Utilities|Array|QuickSort _mystructarray 0 "SortBy_structArray") ; Array Sort By Blueprint Function
    (for (_array_element _array_index) _mystructarray
      (Development|PrintString (Utilities|String|Append (Utilities|String|ToString(Integer) _array_index) ": " (Utilities|String|ToString(Float) (.height _array_element)) ", " (Utilities|String|ToString(Float) (.bodyweight _array_element)) ", " (Utilities|String|ToString(Float) (.score _array_element)))))))

(event Input|KeyboardEvents|4
  (params (Key :type Key%20Structure :default "None"))
  ;[0.0469 0.7135 1] SetTimer Node example: simultaneously controlling the rotation of N actors
  ;;[1 1 1] Rotate spawned Actors
  (:Pressed
    (for _array_element (Variables|SETTIMER|GetMovableActors)
      (bind (_referenceobject _timerhandle) (|SetTimerbyObject _array_element (Math|Random|RandomFloatinRange 0.0 1.0) true)
        (:Then
          (Utilities|Map|Add (Variables|SET_TIMER|GetActorsTimerHandle) _timerhandle _array_element))
        (:OnEvent
          (bind _asactor (Utilities|Casting|CastToActor _referenceobject))
          (Transformation|AddActorLocalRotation _asactor "0.000000,5.000000,0.000000" false false))))))

(fn ConstructionScript)

(fn OnYourTimerFunction
  (Development|PrintString "Call OnTimerFunction" true true "(R=0.016494,G=1.000000,B=0.000000,A=1.000000)"))

(fn SortbyStructArray
  (params (A :type F%20Student%20Structure%20%28by%20ref%29) (B :type F%20Student%20Structure%20%28by%20ref%29))
  ;[1 1 1] Customize a blueprint function for comparing the dimensions of array elements
  (return (> (.Height (Utilities|Struct|BreakFStudent A)) (.Height (Utilities|Struct|BreakFStudent B)))))

(fn SortbyStringArray
  (params (A :type String%20%28by%20ref%29) (B :type String%20%28by%20ref%29))
  ;[1 1 1] Customize a blueprint function for comparing the dimensions of array elements
  (return (> (Utilities|String|Len A) (Utilities|String|Len B))))

(fn SortbyObjectArray
  (params (A :type BP%20My%20Object%20Object%20Reference%20%28by%20ref%29) (B :type BP%20My%20Object%20Object%20Reference%20%28by%20ref%29))
  ;[1 1 1] Customize a blueprint function for comparing the dimensions of array elements
  (return (> (Variables|/Game/Blueprint/BP_MyObject.BP_MyObject_C|GetHealth A) (Variables|/Game/Blueprint/BP_MyObject.BP_MyObject_C|GetHealth B))))

(fn BPNodesExampleAutoGenFunc
  (params (Object :type Object%20Object%20Reference))
  (return false))

(fn BPNodesExampleAutoGenFunc1
  (params (Object :type Object%20Object%20Reference))
  (bind _asactor (Utilities|Casting|CastToActor Object))
  (return (Utilities|Array|ContainsItem (Variables|/Script/Engine.Actor|GetTags _asactor) "YourTag")))

(fn BPNodesExampleAutoGenFunc2
  (params (Object :type Object%20Object%20Reference))
  (bind _asactor (Utilities|Casting|CastToActor Object)
    (:then
      (return (Actor|ActorHasTag _asactor "None")))
    (:CastFailed
      (return false))))